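; Zipline actor that spans a cable between two attach points and lets overlapping actors know when they can use either end.
; On BeginPlay it moves the cable to the start attach point and attaches the cable's end to the end point.
; Start and end collision volumes send SetZiplineMessage through an interact interface, passing which end is enabled plus both attach locations.
; Leaving either volume sends the message with default values, clearing availability; ride movement is left to the receiver.
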(event OnComponentBeginOverlap(EndCollision)
  (params (OverlappedComponent :type Primitive%20Component%20Object%20Reference) (OtherActor :type Actor%20Object%20Reference) (OtherComp :type Primitive%20Component%20Object%20Reference) (OtherBodyIndex :type Integer) (bFromSweep :type Boolean) (SweepResult :type Hit%20Result%20Structure%20%28by%20ref%29))
  ;[1 1 1] Enable Zipline Interaction via BPI Interact Zipline (ZiplineEnd)
  (Class|BPIInteractZipline|SetZipline(Message) OtherActor false true (Transformation|GetWorldLocation (Variables|Default|GetAttachPointStart)) (Transformation|GetWorldLocation (Variables|Default|GetAttachPointEnd))))

(event OnComponentBeginOverlap(StartCollision)
  (params (OverlappedComponent :type Primitive%20Component%20Object%20Reference) (OtherActor :type Actor%20Object%20Reference) (OtherComp :type Primitive%20Component%20Object%20Reference) (OtherBodyIndex :type Integer) (bFromSweep :type Boolean) (SweepResult :type Hit%20Result%20Structure%20%28by%20ref%29))
  ;[1 1 1] Enable Zipline Interaction via BPI Interact Zipline (ZiplineStart)
  (Class|BPIInteractZipline|SetZipline(Message) OtherActor true false (Transformation|GetWorldLocation (Variables|Default|GetAttachPointStart)) (Transformation|GetWorldLocation (Variables|Default|GetAttachPointEnd))))

(event OnComponentEndOverlap(StartCollision)
  (params (OverlappedComponent :type Primitive%20Component%20Object%20Reference) (OtherActor :type Actor%20Object%20Reference) (OtherComp :type Primitive%20Component%20Object%20Reference) (OtherBodyIndex :type Integer))
  ;[1 1 1] Stop The Enable Variable When not in StartCollision
  (Class|BPIInteractZipline|SetZipline(Message) OtherActor false false "0, 0, 0" "0, 0, 0"))

(event OnComponentEndOverlap(EndCollision)
  (params (OverlappedComponent :type Primitive%20Component%20Object%20Reference) (OtherActor :type Actor%20Object%20Reference) (OtherComp :type Primitive%20Component%20Object%20Reference) (OtherBodyIndex :type Integer))
  ;[1 1 1] Stop The Enable Variable When not in StartCollision
  (Class|BPIInteractZipline|SetZipline(Message) OtherActor false false "0, 0, 0" "0, 0, 0"))

(event EventBeginPlay
  ;[1 1 1] Start Function Set Zipline Cable on Begin Play
  (CallFunction|SetZiplineCable))

(fn ConstructionScript)

(fn SetZiplineCable
  ;[1 1 1] Set Cable Attach Point to Attach Point Start
  (Transformation|SetWorldLocation (Variables|Default|GetZiplineCable) (Transformation|GetWorldLocation (Variables|Default|GetAttachPointStart)) false false)
  ;[1 1 1] Set Cable End Attach Point to Attach Point End
  (Class|CableComponent|SetAttachEndtoComponent (Variables|Default|GetZiplineCable) (Variables|Default|GetAttachPointEnd) "None"))