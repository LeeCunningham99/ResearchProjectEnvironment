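; BP_Net is a climbable rope net wall that the third-person character can interact with.
; Its core collision toggles the character's RopeWallInteraction flag on overlap, and hits on the left and right side colliders stop climbing.
; A separate interact collision briefly shows a prompt widget for any overlapping actor.
; Custom events swap the rope material between non-normal and image-normal versions, while the baked and painted normal events are empty.
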(event OnComponentHit(Left)
  (params (HitComponent :type Primitive%20Component%20Object%20Reference) (OtherActor :type Actor%20Object%20Reference) (OtherComp :type Primitive%20Component%20Object%20Reference) (NormalImpulse :type Vector :default "0, 0, 0") (Hit :type Hit%20Result%20Structure%20%28by%20ref%29))
  ;[1 1 1] Stop Climbing At Left/ Right Side Of Wall
  (bind _asbp_third_person_character (Utilities|Casting|CastToBP_ThirdPersonCharacter OtherActor))
  (Default|StopClimbing (stale OnComponentHit(Right) _asbp_third_person_character)))

(event OnComponentHit(Right)
  (params (HitComponent :type Primitive%20Component%20Object%20Reference) (OtherActor :type Actor%20Object%20Reference) (OtherComp :type Primitive%20Component%20Object%20Reference) (NormalImpulse :type Vector :default "0, 0, 0") (Hit :type Hit%20Result%20Structure%20%28by%20ref%29))
  ;[1 1 1] Stop Climbing At Left/ Right Side Of Wall
  (bind _asbp_third_person_character (Utilities|Casting|CastToBP_ThirdPersonCharacter OtherActor))
  (Default|StopClimbing _asbp_third_person_character))

(event OnComponentBeginOverlap(InteractCollision)
  (params (OverlappedComponent :type Primitive%20Component%20Object%20Reference) (OtherActor :type Actor%20Object%20Reference) (OtherComp :type Primitive%20Component%20Object%20Reference) (OtherBodyIndex :type Integer) (bFromSweep :type Boolean) (SweepResult :type Hit%20Result%20Structure%20%28by%20ref%29))
  (bind _widget (Variables|Default|GetWidget))
  ;[1 1 1] Widget Visibility (Press 'KEY' To Interact)
  (Rendering|SetVisibility _widget true false)
  (Utilities|FlowControl|Delay 2.0)
  (Rendering|SetVisibility _widget false false))

(event OnComponentBeginOverlap(CORECOLLISON)
  (params (OverlappedComponent :type Primitive%20Component%20Object%20Reference) (OtherActor :type Actor%20Object%20Reference) (OtherComp :type Primitive%20Component%20Object%20Reference) (OtherBodyIndex :type Integer) (bFromSweep :type Boolean) (SweepResult :type Hit%20Result%20Structure%20%28by%20ref%29))
  (bind _asbp_third_person_character (Utilities|Casting|CastToBP_ThirdPersonCharacter OtherActor))
  (Variables|/Game/ThirdPerson1/Blueprints/BP_ThirdPersonCharacter.BP_ThirdPersonCharacter_C|SetRopeWallInteraction _asbp_third_person_character true))

(event OnComponentEndOverlap(CORECOLLISON)
  (params (OverlappedComponent :type Primitive%20Component%20Object%20Reference) (OtherActor :type Actor%20Object%20Reference) (OtherComp :type Primitive%20Component%20Object%20Reference) (OtherBodyIndex :type Integer))
  (bind _asbp_third_person_character (Utilities|Casting|CastToBP_ThirdPersonCharacter OtherActor))
  (Variables|/Game/ThirdPerson1/Blueprints/BP_ThirdPersonCharacter.BP_ThirdPersonCharacter_C|SetRopeWallInteraction _asbp_third_person_character false))

(event Custom|RopeWallNonNormals
  ;[1 1 1] Non-Normals
  (Rendering|Material|SetMaterial (Variables|Default|GetRope) 0 "/Game/3D-Models/Log_Steps/Rope.Rope"))

(event Custom|RopeWallImageNormals
  ;[1 1 1] Image Normals
  (Rendering|Material|SetMaterial (Variables|Default|GetRope) 0 "/Game/Y2/Models/Materials/NRope.NRope"))

(event Custom|RopeWallBakedNormals)

(event Custom|RopeWallPaintedNormals)

(fn ConstructionScript)