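; BP_Wall_Vert is a vertical moving wall actor whose materials switch between normal-map variants, apparently for comparing techniques.
; Four custom events cover non-normal, image, baked and painted normals.
; Each event sets both material slots on the MovingWallModel mesh, paint and metal in most variants.
; Nothing in this Blueprint calls the events or moves the wall, and BeginPlay, overlap, Tick and the construction script are empty.
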(event Custom|WallVerImageNormals
  (bind _moving_wall_model (Variables|Default|GetMoving_Wall_Model))
  ;[0.3281 0.3281 0.3281] Image Normals
  (Rendering|Material|SetMaterial _moving_wall_model 0 "/Game/Y2/Models/Materials/NBuilding_Door_Paint.NBuilding_Door_Paint")
  (Rendering|Material|SetMaterial _moving_wall_model 1 "/Game/Y2/Models/Materials/NLadder_Rubber.NLadder_Rubber"))

(event Custom|WallVerBakedNormals
  (bind _moving_wall_model (Variables|Default|GetMoving_Wall_Model))
  ;[1 0.1543 0] Baked Normals
  (Rendering|Material|SetMaterial _moving_wall_model 0 "/Game/Y2/Models/Materials/BakedNormals/MovingWalls/N_MWRed_BAKED.N_MWRed_BAKED")
  (Rendering|Material|SetMaterial _moving_wall_model 1 "/Game/Y2/Models/Materials/BakedNormals/MovingWalls/N_MW_Metal_BAKED.N_MW_Metal_BAKED"))

(event Custom|WallVerPaintedNormals
  (bind _moving_wall_model (Variables|Default|GetMoving_Wall_Model))
  ;[0 1 0.001688] Painted Normals
  (Rendering|Material|SetMaterial _moving_wall_model 0 "/Game/Y2/Models/Materials/PaintedNormals/MovingWall/Painted_MWPaint.Painted_MWPaint")
  (Rendering|Material|SetMaterial _moving_wall_model 1 "/Game/Y2/Models/Materials/PaintedNormals/MovingWall/Painted_MWMetal.Painted_MWMetal"))

(event Custom|WallVerNonNormals
  (bind _moving_wall_model (Variables|Default|GetMoving_Wall_Model))
  ;[1 1 1] Non-Normals
  (Rendering|Material|SetMaterial _moving_wall_model 0 "/Game/3D-Models/Moving_Walls/Building_Door_Paint.Building_Door_Paint")
  (Rendering|Material|SetMaterial _moving_wall_model 1 "/Game/3D-Models/Moving_Walls/Building_Door_Metal.Building_Door_Metal"))

(event EventBeginPlay)

(event Collision|EventActorBeginOverlap
  (params (OtherActor :type Actor%20Object%20Reference)))

(event EventTick
  (params (DeltaSeconds :type Float%20%28single-precision%29)))

(fn ConstructionScript)