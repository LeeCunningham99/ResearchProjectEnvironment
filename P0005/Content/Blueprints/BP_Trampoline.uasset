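; Trampoline actor that launches the third-person character upward and can swap between normal-map material variants.
; A hit on its box adds upward velocity to that character via LaunchCharacter and plays a 2D sound for any hitting actor.
; Four custom events reskin the model's three material slots as non-normal, baked, image or painted normals, with painted currently reusing the baked materials.
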(event OnComponentHit(Box)
  (params (HitComponent :type Primitive%20Component%20Object%20Reference) (OtherActor :type Actor%20Object%20Reference) (OtherComp :type Primitive%20Component%20Object%20Reference) (NormalImpulse :type Vector :default "0, 0, 0") (Hit :type Hit%20Result%20Structure%20%28by%20ref%29))
  ;[1 1 1] Trampoline
  (Utilities|FlowControl|Sequence
    (:then_0
      (bind _asbp_third_person_character (Utilities|Casting|CastToBP_ThirdPersonCharacter OtherActor))
      (Character|LaunchCharacter _asbp_third_person_character "0.000000,0.000000,1000.000000" false false))
    (:then_1
      (Audio|PlaySound2D "/Game/SFX/trampoline.trampoline" 1.0 1.0 0.0 0 0))))

(event Custom|TrampolineNonNormals
  (bind _trampoline_model (Variables|Default|GetTrampoline_Model))
  ;[1 1 1] Non-Normals
  (Rendering|Material|SetMaterial _trampoline_model 0 "/Game/3D-Models/Trampoline/Trampline_Metal.Trampline_Metal")
  (Rendering|Material|SetMaterial _trampoline_model 1 "/Game/3D-Models/Trampoline/Trampoline_Mesh.Trampoline_Mesh")
  (Rendering|Material|SetMaterial _trampoline_model 2 "/Game/3D-Models/Trampoline/Trampoline_Tarp.Trampoline_Tarp"))

(event Custom|TrampolineBakedNormals
  (bind _trampoline_model (Variables|Default|GetTrampoline_Model))
  ;[1 0.1543 0] Baked Normals
  (Rendering|Material|SetMaterial _trampoline_model 0 "/Game/Y2/Models/Materials/BakedNormals/Trampoline/N_TrampolineMetal_BAKED.N_TrampolineMetal_BAKED")
  (Rendering|Material|SetMaterial _trampoline_model 1 "/Game/Y2/Models/Materials/BakedNormals/Trampoline/N_TrampolineMesh_BAKED.N_TrampolineMesh_BAKED")
  (Rendering|Material|SetMaterial _trampoline_model 2 "/Game/Y2/Models/Materials/BakedNormals/Trampoline/N_TrampolineTarp_BAKED.N_TrampolineTarp_BAKED"))

(event Custom|TrampolinePaintedNormals
  (bind _trampoline_model (Variables|Default|GetTrampoline_Model))
  ;[0 1 0.001688] Painted Normals
  (Rendering|Material|SetMaterial _trampoline_model 0 "/Game/Y2/Models/Materials/BakedNormals/Trampoline/N_TrampolineMetal_BAKED.N_TrampolineMetal_BAKED")
  (Rendering|Material|SetMaterial _trampoline_model 1 "/Game/Y2/Models/Materials/BakedNormals/Trampoline/N_TrampolineMesh_BAKED.N_TrampolineMesh_BAKED")
  (Rendering|Material|SetMaterial _trampoline_model 2 "/Game/Y2/Models/Materials/BakedNormals/Trampoline/N_TrampolineTarp_BAKED.N_TrampolineTarp_BAKED"))

(event Custom|TrampolineImageNormals
  (bind _trampoline_model (Variables|Default|GetTrampoline_Model))
  ;[0.3281 0.3281 0.3281] Image Normals
  (Rendering|Material|SetMaterial _trampoline_model 0 "/Game/Y2/Models/Materials/NMetal.NMetal")
  (Rendering|Material|SetMaterial _trampoline_model 1 "/Game/Y2/Models/Materials/NTrampoline_Mesh.NTrampoline_Mesh")
  (Rendering|Material|SetMaterial _trampoline_model 2 "/Game/Y2/Models/Materials/NTrampoline_Tarp.NTrampoline_Tarp"))

(fn ConstructionScript)