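; BP_Rope is a rope prop that flags BP_ThirdPersonCharacter for ladder-style rope movement and animation.
; Box overlap sets those character flags and adds rope audio; leaving clears them, restores Walking mode and stops the audio.
; A separate Collision overlap briefly shows an interact widget.
; Four custom events swap both mesh materials between non-normal, baked, image and painted normal variants.
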(event OnComponentBeginOverlap(Collision)
  (params (OverlappedComponent :type Primitive%20Component%20Object%20Reference) (OtherActor :type Actor%20Object%20Reference) (OtherComp :type Primitive%20Component%20Object%20Reference) (OtherBodyIndex :type Integer) (bFromSweep :type Boolean) (SweepResult :type Hit%20Result%20Structure%20%28by%20ref%29))
  (bind _widget (Variables|Default|GetWidget))
  ;[1 1 1] Interact Widget
  (Rendering|SetVisibility _widget true false)
  (Utilities|FlowControl|Delay 2.0)
  (Rendering|SetVisibility _widget false false))

(event OnComponentBeginOverlap(Box)
  (params (OverlappedComponent :type Primitive%20Component%20Object%20Reference) (OtherActor :type Actor%20Object%20Reference) (OtherComp :type Primitive%20Component%20Object%20Reference) (OtherBodyIndex :type Integer) (bFromSweep :type Boolean) (SweepResult :type Hit%20Result%20Structure%20%28by%20ref%29))
  ;[1 1 1] Collision Begin
  (Utilities|FlowControl|Sequence
    (:then_0
      (bind _asbp_third_person_character (Utilities|Casting|CastToBP_ThirdPersonCharacter OtherActor))
      (Variables|/Game/ThirdPerson1/Blueprints/BP_ThirdPersonCharacter.BP_ThirdPersonCharacter_C|SetNearLadder? _asbp_third_person_character true)
      (Variables|/Game/ThirdPerson1/Blueprints/BP_ThirdPersonCharacter.BP_ThirdPersonCharacter_C|SetRopeAnim _asbp_third_person_character true))
    (:then_1
      (if (Variables|/Game/ThirdPerson1/Blueprints/BP_ThirdPersonCharacter.BP_ThirdPersonCharacter_C|GetNearLadder? _asbp_third_person_character)
        (bind _returnvalue (AddComponent|AddAudioComponent false))
        (Variables|Default|SetStopPlayingRopeAudio _returnvalue)))))

(event OnComponentEndOverlap(Box)
  (params (OverlappedComponent :type Primitive%20Component%20Object%20Reference) (OtherActor :type Actor%20Object%20Reference) (OtherComp :type Primitive%20Component%20Object%20Reference) (OtherBodyIndex :type Integer))
  (bind _stopplayingropeaudio (Variables|Default|GetStopPlayingRopeAudio))
  ;[1 1 1] Collisions End
  (Utilities|FlowControl|Sequence
    (:then_0
      (bind _asbp_third_person_character (Utilities|Casting|CastToBP_ThirdPersonCharacter OtherActor))
      (Variables|/Game/ThirdPerson1/Blueprints/BP_ThirdPersonCharacter.BP_ThirdPersonCharacter_C|SetNearLadder? _asbp_third_person_character false)
      (Variables|/Game/ThirdPerson1/Blueprints/BP_ThirdPersonCharacter.BP_ThirdPersonCharacter_C|SetLadder _asbp_third_person_character false)
      (Variables|/Game/ThirdPerson1/Blueprints/BP_ThirdPersonCharacter.BP_ThirdPersonCharacter_C|SetRopeAnim _asbp_third_person_character false)
      (Pawn|Components|CharacterMovement|SetMovementMode (Variables|/Script/Engine.Character|GetCharacterMovement _asbp_third_person_character) "MOVE_Walking" 0))
    (:then_1
      (Audio|Components|Audio|FadeOut _stopplayingropeaudio 4.0 0.0 "Linear" :!class /Script/Engine.AudioComponent)
      (Audio|Components|Audio|Stop _stopplayingropeaudio))))

(event Custom|RopeNonNormals
  (bind _rope_model (Variables|Default|GetRope_Model))
  ;[1 1 1] Non-Normals
  (Rendering|Material|SetMaterial _rope_model 0 "/Game/3D-Models/Log_Steps/Rope.Rope")
  (Rendering|Material|SetMaterial _rope_model 1 "/Game/3D-Models/Log_Steps/Rope_Metal.Rope_Metal"))

(event Custom|RopeBakedNormals
  (bind _rope_model (Variables|Default|GetRope_Model))
  ;[1 0.1543 0] Baked Normals
  (Rendering|Material|SetMaterial _rope_model 0 "/Game/Y2/Models/Materials/BakedNormals/Rope/N_Rope_BAKED.N_Rope_BAKED")
  (Rendering|Material|SetMaterial _rope_model 1 "/Game/Y2/Models/Materials/BakedNormals/Rope/N_RopeMetal_BAKED.N_RopeMetal_BAKED"))

(event Custom|RopePaintedNormals
  (bind _rope_model (Variables|Default|GetRope_Model))
  ;[0 1 0.001688] Painted Normals
  (Rendering|Material|SetMaterial _rope_model 0 "/Game/Y2/Models/Materials/PaintedNormals/Rope/Painted_Rope.Painted_Rope")
  (Rendering|Material|SetMaterial _rope_model 1 "/Game/Y2/Models/Materials/PaintedNormals/Rope/Painted_RopeMetal.Painted_RopeMetal"))

(event Custom|RopeImageNormals
  (bind _rope_model (Variables|Default|GetRope_Model))
  ;[0.3281 0.3281 0.3281] Image Normals
  (Rendering|Material|SetMaterial _rope_model 0 "/Game/Y2/Models/Materials/NRope.NRope")
  (Rendering|Material|SetMaterial _rope_model 1 "/Game/Y2/Models/Materials/NRope_Metal.NRope_Metal"))

(event EventBeginPlay)

(event EventTick
  (params (DeltaSeconds :type Float%20%28single-precision%29)))

(fn ConstructionScript)