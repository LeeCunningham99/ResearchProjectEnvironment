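; BP_Ladder is a ladder actor that tells BP_ThirdPersonCharacter when it is within climbing range.
; Entering the Box sets the character's NearLadder and LadderAnim flags and adds a ladder audio component.
; Leaving clears those flags and Ladder, restores Walking movement, and calls FadeOut then an immediate Stop on the audio.
; A separate WidgetCollison overlap briefly shows an interact widget, hiding it after a delay.
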(event OnComponentBeginOverlap(Box)
  (params (OverlappedComponent :type Primitive%20Component%20Object%20Reference) (OtherActor :type Actor%20Object%20Reference) (OtherComp :type Primitive%20Component%20Object%20Reference) (OtherBodyIndex :type Integer) (bFromSweep :type Boolean) (SweepResult :type Hit%20Result%20Structure%20%28by%20ref%29))
  ;[1 1 1] Collision Begin
  (Utilities|FlowControl|Sequence
    (:then_0
      (bind _asbp_third_person_character (Utilities|Casting|CastToBP_ThirdPersonCharacter OtherActor))
      (Variables|/Game/ThirdPerson1/Blueprints/BP_ThirdPersonCharacter.BP_ThirdPersonCharacter_C|SetNearLadder? _asbp_third_person_character true)
      (Variables|/Game/ThirdPerson1/Blueprints/BP_ThirdPersonCharacter.BP_ThirdPersonCharacter_C|SetLadderAnim _asbp_third_person_character true))
    (:then_1
      (if (Variables|/Game/ThirdPerson1/Blueprints/BP_ThirdPersonCharacter.BP_ThirdPersonCharacter_C|GetNearLadder? _asbp_third_person_character)
        (bind _returnvalue (AddComponent|AddAudioComponent false))
        (Variables|Default|SetStopPlayingLadderAudio _returnvalue)))))

(event OnComponentEndOverlap(Box)
  (params (OverlappedComponent :type Primitive%20Component%20Object%20Reference) (OtherActor :type Actor%20Object%20Reference) (OtherComp :type Primitive%20Component%20Object%20Reference) (OtherBodyIndex :type Integer))
  (bind _stopplayingladderaudio (Variables|Default|GetStopPlayingLadderAudio))
  ;[1 1 1] Collision End
  (Utilities|FlowControl|Sequence
    (:then_0
      (bind _asbp_third_person_character (Utilities|Casting|CastToBP_ThirdPersonCharacter OtherActor))
      (Variables|/Game/ThirdPerson1/Blueprints/BP_ThirdPersonCharacter.BP_ThirdPersonCharacter_C|SetNearLadder? _asbp_third_person_character false)
      (Variables|/Game/ThirdPerson1/Blueprints/BP_ThirdPersonCharacter.BP_ThirdPersonCharacter_C|SetLadder _asbp_third_person_character false)
      (Variables|/Game/ThirdPerson1/Blueprints/BP_ThirdPersonCharacter.BP_ThirdPersonCharacter_C|SetLadderAnim _asbp_third_person_character false)
      (Pawn|Components|CharacterMovement|SetMovementMode (Variables|/Script/Engine.Character|GetCharacterMovement _asbp_third_person_character) "MOVE_Walking" 0))
    (:then_1
      (Audio|Components|Audio|FadeOut _stopplayingladderaudio 4.0 0.0 "Linear" :!class /Script/Engine.AudioComponent)
      (Audio|Components|Audio|Stop _stopplayingladderaudio))))

(event OnComponentBeginOverlap(WidgetCollison)
  (params (OverlappedComponent :type Primitive%20Component%20Object%20Reference) (OtherActor :type Actor%20Object%20Reference) (OtherComp :type Primitive%20Component%20Object%20Reference) (OtherBodyIndex :type Integer) (bFromSweep :type Boolean) (SweepResult :type Hit%20Result%20Structure%20%28by%20ref%29))
  (bind _widget (Variables|Default|GetWidget))
  ;[1 1 1] Interact Widget
  (Rendering|SetVisibility _widget true false)
  (Utilities|FlowControl|Delay 2.0)
  (Rendering|SetVisibility _widget false false))

(event EventBeginPlay)

(event Collision|EventActorBeginOverlap
  (params (OtherActor :type Actor%20Object%20Reference)))

(event EventTick
  (params (DeltaSeconds :type Float%20%28single-precision%29)))

(fn ConstructionScript)