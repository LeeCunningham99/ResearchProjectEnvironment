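; Thin horizontal platform Blueprint whose model switches between material sets that compare normal-map approaches.
; Four custom events (baked, none, image and painted normals) each set both material slots on PlatformModel.
; The painted event currently assigns the same baked materials as the baked event.
; It has no movement or gameplay logic of its own, and its construction script is empty.
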(event Custom|TPlatHorImageNormals
  (bind _platform_model (Variables|Default|GetPlatform_Model))
  ;[0.3281 0.3281 0.3281] Image Normals
  (Rendering|Material|SetMaterial _platform_model 0 "/Game/Y2/Models/Materials/NSliding_Platform_Metal_Light.NSliding_Platform_Metal_Light")
  (Rendering|Material|SetMaterial _platform_model 1 "/Game/Y2/Models/Materials/NMetal.NMetal"))

(event Custom|TPlatHorNonNormals
  (bind _platform_model (Variables|Default|GetPlatform_Model))
  ;[1 1 1] Non-Normals
  (Rendering|Material|SetMaterial _platform_model 0 "/Game/3D-Models/Sliding_Platform/Sliding_Platform_Metal_Light.Sliding_Platform_Metal_Light")
  (Rendering|Material|SetMaterial _platform_model 1 "/Game/3D-Models/Sliding_Platform/Sliding_Platform_Metal.Sliding_Platform_Metal"))

(event Custom|TPlatHorBakedNormals
  (bind _platform_model (Variables|Default|GetPlatform_Model))
  ;[1 0.1543 0] Baked Normals
  (Rendering|Material|SetMaterial _platform_model 0 "/Game/Y2/Models/Materials/BakedNormals/SlidingPlatform/N_SlidingPlatformLightMetal_BAKED.N_SlidingPlatformLightMetal_BAKED")
  (Rendering|Material|SetMaterial _platform_model 1 "/Game/Y2/Models/Materials/BakedNormals/SlidingPlatform/N_SlidingPlatformMetal_BAKED.N_SlidingPlatformMetal_BAKED"))

(event Custom|TPlatHorPaintedNormals
  (bind _platform_model (Variables|Default|GetPlatform_Model))
  ;[0 1 0.001688] Painted Normals
  (Rendering|Material|SetMaterial _platform_model 0 "/Game/Y2/Models/Materials/BakedNormals/SlidingPlatform/N_SlidingPlatformLightMetal_BAKED.N_SlidingPlatformLightMetal_BAKED")
  (Rendering|Material|SetMaterial _platform_model 1 "/Game/Y2/Models/Materials/BakedNormals/SlidingPlatform/N_SlidingPlatformMetal_BAKED.N_SlidingPlatformMetal_BAKED"))

(event EventBeginPlay)

(event Collision|EventActorBeginOverlap
  (params (OtherActor :type Actor%20Object%20Reference)))

(event EventTick
  (params (DeltaSeconds :type Float%20%28single-precision%29)))

(fn ConstructionScript)