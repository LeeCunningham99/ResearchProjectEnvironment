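; Zipline actor with an editable end point; its construction script stretches a collision spline between the start and end sockets and builds an offset spline mesh along it.
; A helper estimates the grab point by travelling along the cable direction by the player's horizontal distance from the start.
; Cable attachment, overlap binding, player notification and polling timers are present but unwired, leaving runtime events empty apart from the interface call that clears both timers.
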(event Custom|On%20Player%20Detected
  (params (OverlappedComponent :type Primitive%20Component%20Object%20Reference) (OtherActor :type Actor%20Object%20Reference) (OtherComp :type Primitive%20Component%20Object%20Reference) (OtherBodyIndex :type Integer) (bFromSweep :type Boolean) (SweepResult :type Hit%20Result%20Structure%20%28by%20ref%29)))

(event Custom|Stop%20Checking%20For%20Player
  (params (OverlappedComponent :type Primitive%20Component%20Object%20Reference) (OtherActor :type Actor%20Object%20Reference) (OtherComp :type Primitive%20Component%20Object%20Reference) (OtherBodyIndex :type Integer)))

(event Custom|Set%20Current%20Target)

(event Custom|Check%20Distance)

(event EventBeginPlay
  ;[1 1 1] Set Cable Points
)

(fn ConstructionScript
  (bind _returnvalue (Math|Float|MakeLiteralFloat -1.3e+02))
  (bind _spline_collision (Variables|Default|GetSpline_Collision))
  (bind _spline_collision_2 (Variables|Default|GetSpline_Collision))
  ;[1 1 1] Set Zipline Endpoint
  (Transformation|SetRelativeLocation (Variables|Default|GetZipline_End) (Variables|Default|GetEnd_Point) false false)
  ;[1 1 1] Set Spline Position Inbetween Zipline Endpoints - For collsion box
  (Spline|SetLocationatSplinePoint (Variables|Default|GetSpline_Collision) 0 (Transformation|GetSocketLocation (Variables|Default|GetZipline_Start) (Variables|Default|GetIn%20Socket%20Name)) "World" true)
  (Spline|SetLocationatSplinePoint (Variables|Default|GetSpline_Collision) 1 (Transformation|GetSocketLocation (Variables|Default|GetZipline_End) (Variables|Default|GetIn%20Socket%20Name)) "World" true)
  (for _index (range 0 (- (Spline|GetNumberOfSplinePoints (Variables|Default|GetSpline_Collision)) 2))
    (bind _returnvalue_2 (AddComponent|AddSplineMeshComponent false))
    (Variables|Default|SetCable_Collision _returnvalue_2)
    (SplineMesh|SetStartandEnd _returnvalue_2 (- (Spline|GetLocationatSplinePoint _spline_collision_2 _index "Local") (Math|Vector|MakeVector 0.0 0.0 _returnvalue)) (Spline|GetLocationatSplinePoint _spline_collision_2 _index "Local") (- (Spline|GetLocationatSplinePoint _spline_collision (+ _index 1) "Local") (Math|Vector|MakeVector 0.0 0.0 _returnvalue)) (Spline|GetLocationatSplinePoint _spline_collision (+ _index 1) "Local") true :!class /Script/Engine.SplineMeshComponent)))

(fn GetStartandEndSockets
  (return (Transformation|GetSocketLocation (Variables|Default|GetZipline_Start) (Variables|Default|GetIn%20Socket%20Name)) (Transformation|GetSocketLocation (Variables|Default|GetZipline_End) (Variables|Default|GetIn%20Socket%20Name))))

(fn PointOfZiplineInteraction
  (params (self2 :type Actor%20Object%20Reference))
  (bind (_start_socket _end_socket) (CallFunction|GetStartandEndSockets))
  (bind _returnvalue (Transformation|GetActorLocation self2))
  (bind _in_socket_name (Variables|Default|GetIn%20Socket%20Name))
  (bind _zipline_start (Variables|Default|GetZipline_Start))
  (bind _returnvalue_2 (Transformation|GetSocketLocation _zipline_start _in_socket_name))
  (return (+ (* (Math|Vector|GetUnitDirection(Vector) _start_socket _end_socket) (Math|Vector|VectorLength (- (Math|Vector|MakeVector (.x _returnvalue) (.y _returnvalue) 0.0) (Math|Vector|MakeVector (.x _returnvalue_2) (.y _returnvalue_2) 0.0)))) (.Start%20Socket (CallFunction|GetStartandEndSockets)))))