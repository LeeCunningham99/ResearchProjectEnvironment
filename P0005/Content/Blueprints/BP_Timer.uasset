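; BP_Timer is an actor that works as a clock, showing the current time from Now as hours, minutes and seconds.
; Every Tick it reads the 12-hour hour, minute and second, converts each to text and writes it to the Hour, Minute and Second text elements.
; Despite its name it does no countdown or elapsed-time tracking, and its other events and construction script are empty.
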(event EventBeginPlay)

(event Collision|EventActorBeginOverlap
  (params (OtherActor :type Actor%20Object%20Reference)))

(event EventTick
  (params (DeltaSeconds :type Float%20%28single-precision%29))
  (bind _returnvalue (Math|DateTime|Now))
  (bind _output_get (Variables|Default|SetHours (Class|KismetMathLibrary|GetHour12 _returnvalue)))
  (bind _output_get_2 (Variables|Default|SetMinutes (Class|KismetMathLibrary|GetMinute _returnvalue)))
  (bind _output_get_3 (Variables|Default|SetSeconds (Class|KismetMathLibrary|GetSecond _returnvalue)))
  (Rendering|Components|TextRender|SetText (Variables|Default|GetHour) (Utilities|Text|ToText(Integer) _output_get))
  (Rendering|Components|TextRender|SetText (Variables|Default|GetMinute) (Utilities|Text|ToText(Integer) _output_get_2))
  (Rendering|Components|TextRender|SetText (Variables|Default|GetSecond) (Utilities|Text|ToText(Integer) _output_get_3)))

(fn ConstructionScript)