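; Third-person game mode that respawns the player and persists a high score between sessions.
; RespawnPlayer destroys the current character, then spawns and possesses a new one at the last checkpoint, or at a fixed fallback location if none is valid.
; BeginPlay loads the high score from a Score_Save slot, creating a save if missing, and EndPlay writes it back.
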(event Custom|Respawn%20Player
  ;[1 1 1] Respawn Player At Previous Checkpoint
  (Actor|DestroyActor (Game|GetPlayerCharacter 0))
  (bind _last_checkpoint (Variables|Default|GetLast%20Checkpoint)
    (:then
      (bind _returnvalue (Game|SpawnActorfromClass "/Game/ThirdPerson1/Blueprints/BP_ThirdPersonCharacter.BP_ThirdPersonCharacter_C" (Math|Transform|MakeTransform (.location (Transformation|GetWorldTransform (Variables|/Game/Blueprints/BP_Checkpoint.BP_Checkpoint_C|GetPOS _last_checkpoint))) (.rotation (Transformation|GetWorldTransform (Variables|/Game/Blueprints/BP_Checkpoint.BP_Checkpoint_C|GetPOS _last_checkpoint))) "1.000000,1.000000,1.000000") "AlwaysSpawn" "MultiplyWithRoot" 0 0))
      (Pawn|Possess (Game|GetPlayerController 0) _returnvalue))
    (:else
      (bind _returnvalue_2 (Game|SpawnActorfromClass "/Game/ThirdPerson1/Blueprints/BP_ThirdPersonCharacter.BP_ThirdPersonCharacter_C" (Math|Transform|MakeTransform "100.000000,100.000000,100.000000" "0, 0, 0" "1.000000,1.000000,1.000000") "AlwaysSpawn" "MultiplyWithRoot" 0 0))
      (Pawn|Possess (Game|GetPlayerController 0) _returnvalue_2))))

(event EventEndPlay
  (params (EndPlayReason :type EEndPlayReason%20Enum :default "Destroyed"))
  ;[1 1 1] Save and Load Game
  (CallFunction|SaveGame))

(event EventBeginPlay
  ;[1 1 1] Save and Load Game
  (CallFunction|LoadGame))

(fn ConstructionScript)

(fn SaveGame
  ;[1 1 1] Create a save game
  (bind _returnvalue (SaveGame|CreateSaveGameObject "/Game/Blueprints/Score_Save.Score_Save_C"))
  (bind _output_get (Variables|Default|SetSave%20Ref _returnvalue))
  (bind _asscore_save (Utilities|Casting|CastToScore_Save _output_get))
  (Variables|/Game/Blueprints/Score_Save.Score_Save_C|SetHigh%20Score _asscore_save (Variables|Default|GetHigh%20Score))
  (SaveGame|SaveGametoSlot (Variables|Default|GetSave%20Ref) (Variables|Default|GetSlot%20Name)))

(fn LoadGame
  ;[1 1 1] Load game then save // Save game
  (bind _returnvalue (SaveGame|DoesSaveGameExist (Variables|Default|GetSlot%20Name)))
  (if _returnvalue
    (bind _returnvalue_2 (SaveGame|LoadGamefromSlot (Variables|Default|GetSlot%20Name)))
    (bind _output_get (Variables|Default|SetSave%20Ref _returnvalue_2))
    (bind _asscore_save (Utilities|Casting|CastToScore_Save _output_get))
    (Variables|Default|SetHigh%20Score (Variables|/Game/Blueprints/Score_Save.Score_Save_C|GetHigh%20Score _asscore_save))
    (SaveGame|SaveGametoSlot (Variables|Default|GetSave%20Ref) (Variables|Default|GetSlot%20Name))
    (else
      (CallFunction|SaveGame))))