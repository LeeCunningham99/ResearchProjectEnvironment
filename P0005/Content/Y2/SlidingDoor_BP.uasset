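; Sliding door actor that slides its LeftDoor component along the world Z axis when OpenSlidingDoor is called.
; A DoOnce captures the door's starting location, then the SlidingDoor timeline adds its value to that Z position each update.
; BeginPlay caches a first-person character reference that the graph never reads.
; The Interact event is empty, and the button animation and debug prints are disconnected leftovers.
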(event Custom|OpenSlidingDoor
  ;[1 1 1] Sliding Door Button Interaction
  ;;[1 1 1] Sliding Door Animation
  (Utilities|FlowControl|DoOnce false
    (:Completed
      (Variables|Default|SetInitialDoorPos (Transformation|GetWorldLocation (Variables|Default|GetLeftDoor)))
      (bind _slidingdoor (Timeline|SlidingDoor Play)
        (:Update
          (Transformation|SetWorldLocation (Variables|Default|GetLeftDoor) (Math|Vector|MakeVector (.x (Variables|Default|GetInitialDoorPos)) (.y (Variables|Default|GetInitialDoorPos)) (+ (.z (Variables|Default|GetInitialDoorPos)) _slidingdoor)) false false))))))

(event EventBeginPlay
  ;[1 1 1] Reference To First Person Character. IS THIS NEEDED?
  (bind _asbp_first_person_character (Utilities|Casting|CastToBP_FirstPersonCharacter (Game|GetPlayerCharacter 0)))
  (Variables|Default|SetCharRef _asbp_first_person_character))

(event EventInteract
  ;[1 1 1] Sliding Door Button Interaction
  ;;[1 1 1] Sliding Door Animation
)

(fn ConstructionScript)