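; Lamp actor that switches the materials on a group of lamp static meshes to compare normal-map variants.
; Custom events LampNonNormals and LampImageNormals set each mesh's metal and glass slots to either the plain materials or their N-prefixed counterparts.
; The painted and baked normal events are empty stubs, and nothing runs on BeginPlay or Tick.
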(event Custom|LampNonNormals
  (bind _lamp_v7_staticmeshcomponent0 (Variables|Default|GetLamp_V7_StaticMeshComponent0))
  ;[1 1 1] Non-Normals
  (Rendering|Material|SetMaterial _lamp_v7_staticmeshcomponent0 0 "/Game/3D-Models/Lamp/Metal.Metal")
  (Rendering|Material|SetMaterial _lamp_v7_staticmeshcomponent0 1 "/Game/3D-Models/Lamp/Glass.Glass")
  (Rendering|Material|SetMaterial _lamp_v7_staticmeshcomponent0 2 "/Game/3D-Models/Lamp/Metal.Metal"))

(event Custom|LampImageNormals
  (bind _lamp_v7_staticmeshcomponent0 (Variables|Default|GetLamp_V7_StaticMeshComponent0))
  ;[1 1 1] Image Normals
  (Rendering|Material|SetMaterial _lamp_v7_staticmeshcomponent0 0 "/Game/Y2/Models/Materials/NMetal.NMetal")
  (Rendering|Material|SetMaterial _lamp_v7_staticmeshcomponent0 1 "/Game/Y2/Models/Materials/NGlass.NGlass")
  (Rendering|Material|SetMaterial _lamp_v7_staticmeshcomponent0 2 "/Game/Y2/Models/Materials/NMetal.NMetal"))

(event Custom|LampBakedNormals)

(event Custom|LampPaintedNormals)

(event EventBeginPlay)

(event Collision|EventActorBeginOverlap
  (params (OtherActor :type Actor%20Object%20Reference)))

(event EventTick
  (params (DeltaSeconds :type Float%20%28single-precision%29)))

(fn ConstructionScript)