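; Danger sign actor that switches its materials between normal-map variants, apparently for comparing normal mapping techniques.
; Custom events set both material slots, metal and sign face, on four static mesh components at once.
; The Non-Normals event applies the plain materials and the Image Normals event applies their N-prefixed counterparts.
; Baked and Painted Normals events are empty stubs, and nothing in this Blueprint calls the events.
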(event Custom|DangerSTNonNormals
  ;[1 1 1] Non-Normals
  (Rendering|Material|SetMaterial (Variables|Default|GetDangerSignT_StaticMeshComponent1) 0 "/Game/3D-Models/Signs/SignMetal.SignMetal")
  (Rendering|Material|SetMaterial (Variables|Default|GetDangerSignT_StaticMeshComponent1) 1 "/Game/3D-Models/Signs/Danger2.Danger2"))

(event Custom|DangerSTImageNormals
  ;[1 1 1] Image Normals
  (Rendering|Material|SetMaterial (Variables|Default|GetDangerSignT_StaticMeshComponent1) 0 "/Game/Y2/Models/Materials/NSignMetal.NSignMetal")
  (Rendering|Material|SetMaterial (Variables|Default|GetDangerSignT_StaticMeshComponent1) 1 "/Game/Y2/Models/Materials/NDanger2.NDanger2"))

(event Custom|DangerSTBakedNormals)

(event Custom|DangerSTPaintedNormals)

(event EventBeginPlay)

(event Collision|EventActorBeginOverlap
  (params (OtherActor :type Actor%20Object%20Reference)))

(event EventTick
  (params (DeltaSeconds :type Float%20%28single-precision%29)))

(fn ConstructionScript)