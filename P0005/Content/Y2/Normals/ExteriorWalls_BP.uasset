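; Exterior walls Blueprint that switches a set of building wall meshes between four normal-map material variants.
; Four custom events apply the variants: non-normals, image normals, baked normals and painted normals.
; Each sets slot 0 to an exterior material and slot 1 to an interior material on the same hardcoded wall and half-wall component list.
; Nothing here calls these events; BeginPlay, Tick and the construction script are empty.
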(event Custom|EWNonNormals
  ;[1 1 1] Non-Normals
  (Rendering|Material|SetMaterial (Variables|Default|GetBuilding_Wall53_StaticMeshComponent0) 0 "/Game/3D-Models/Building/Building_Wall_Exterior.Building_Wall_Exterior")
  (Rendering|Material|SetMaterial (Variables|Default|GetBuilding_Wall53_StaticMeshComponent0) 1 "/Game/3D-Models/Building/Building_Wall_Interior.Building_Wall_Interior"))

(event Custom|EWBakedNormals
  ;[1 0.1543 0] Baked Normals
  (Rendering|Material|SetMaterial (Variables|Default|GetBuilding_Wall53_StaticMeshComponent0) 0 "/Game/Y2/Models/Materials/BakedNormals/Wall/N_Bricks_BAKED.N_Bricks_BAKED")
  (Rendering|Material|SetMaterial (Variables|Default|GetBuilding_Wall53_StaticMeshComponent0) 1 "/Game/Y2/Models/Materials/BakedNormals/Wall/N_WallInterior_BAKED.N_WallInterior_BAKED"))

(event Custom|EWPaintedNormals
  ;[0 1 0.001688] Painted Normals
  (Rendering|Material|SetMaterial (Variables|Default|GetBuilding_Wall53_StaticMeshComponent0) 0 "/Game/Y2/Models/Materials/PaintedNormals/BuildingWallExterior/Painted_ExteriorWall.Painted_ExteriorWall")
  (Rendering|Material|SetMaterial (Variables|Default|GetBuilding_Wall53_StaticMeshComponent0) 1 "/Game/Y2/Models/Materials/PaintedNormals/BuildingWallExterior/Painted_InteriorWall.Painted_InteriorWall"))

(event Custom|EWImageNormals
  ;[0.3281 0.3281 0.3281] Image Normals
  (Rendering|Material|SetMaterial (Variables|Default|GetBuilding_Wall53_StaticMeshComponent0) 0 "/Game/Y2/Models/Materials/NBuilding_Wall_Exterior.NBuilding_Wall_Exterior")
  (Rendering|Material|SetMaterial (Variables|Default|GetBuilding_Wall53_StaticMeshComponent0) 1 "/Game/Y2/Models/Materials/NBuilding_Wall_Interior.NBuilding_Wall_Interior"))

(event EventBeginPlay)

(event Collision|EventActorBeginOverlap
  (params (OtherActor :type Actor%20Object%20Reference)))

(event EventTick
  (params (DeltaSeconds :type Float%20%28single-precision%29)))

(fn ConstructionScript)