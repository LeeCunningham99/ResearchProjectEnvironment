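; Blueprint grouping Gleditsia-style tree meshes (Tree4) whose materials switch between normal-map variants.
; The Tree4NonNormals and Tree4ImageNormals events set all five material slots on every tree mesh component to the plain or normal-mapped material set.
; Tree4BakedNormals and Tree4PaintedNormals are empty stubs, and nothing in this Blueprint calls any of these events.
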(event Custom|Tree4NonNormals
  ;[1 1 1] Non-Normals
  (Rendering|Material|SetMaterial (Variables|Default|Get4Gledista_Triacanthos_60_StaticMeshComponent0) 0 "/Game/3D-Models/Tree/Material__1.Material__1")
  (Rendering|Material|SetMaterial (Variables|Default|Get4Gledista_Triacanthos_60_StaticMeshComponent0) 1 "/Game/3D-Models/Tree/Material__2.Material__2")
  (Rendering|Material|SetMaterial (Variables|Default|Get4Gledista_Triacanthos_60_StaticMeshComponent0) 2 "/Game/3D-Models/Tree/Material__3.Material__3")
  (Rendering|Material|SetMaterial (Variables|Default|Get4Gledista_Triacanthos_60_StaticMeshComponent0) 3 "/Game/3D-Models/Tree/Material__4.Material__4")
  (Rendering|Material|SetMaterial (Variables|Default|Get4Gledista_Triacanthos_60_StaticMeshComponent0) 4 "/Game/3D-Models/Tree/Material__0.Material__0"))

(event Custom|Tree4ImageNormals
  ;[1 1 1] Image Normals
  (Rendering|Material|SetMaterial (Variables|Default|Get4Gledista_Triacanthos_60_StaticMeshComponent0) 0 "/Game/Y2/Models/Materials/NMaterial__1.NMaterial__1")
  (Rendering|Material|SetMaterial (Variables|Default|Get4Gledista_Triacanthos_60_StaticMeshComponent0) 1 "/Game/Y2/Models/Materials/NMaterial__2.NMaterial__2")
  (Rendering|Material|SetMaterial (Variables|Default|Get4Gledista_Triacanthos_60_StaticMeshComponent0) 2 "/Game/Y2/Models/Materials/NMaterial__3.NMaterial__3")
  (Rendering|Material|SetMaterial (Variables|Default|Get4Gledista_Triacanthos_60_StaticMeshComponent0) 3 "/Game/Y2/Models/Materials/NMaterial__4.NMaterial__4")
  (Rendering|Material|SetMaterial (Variables|Default|Get4Gledista_Triacanthos_60_StaticMeshComponent0) 4 "/Game/Y2/Models/Materials/NMaterial__0.NMaterial__0"))

(event Custom|Tree4BakedNormals)

(event Custom|Tree4PaintedNormals)

(event EventBeginPlay)

(event Collision|EventActorBeginOverlap
  (params (OtherActor :type Actor%20Object%20Reference)))

(event EventTick
  (params (DeltaSeconds :type Float%20%28single-precision%29)))

(fn ConstructionScript)