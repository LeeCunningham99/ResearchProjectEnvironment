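; Building floor Blueprint that switches its many floor mesh components between normal map variants, apparently for comparing techniques.
; Four custom events set material slot 0 on the same hard-wired component list to the non-normal, image, baked or painted material.
; Nothing in this Blueprint calls these events, so switching relies on outside callers.
; BeginPlay, overlap, Tick and the construction script are empty.
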(event Custom|BFNonNormals
  ;[1 1 1] Non-Normals
  (Rendering|Material|SetMaterial (Variables|Default|GetBuilding_Floor28_StaticMeshComponent0) 0 "/Game/3D-Models/Building/Building_Floor1.Building_Floor1"))

(event Custom|BFPaintedNormals
  ;[0 1 0.001688] Painted Normals
  (Rendering|Material|SetMaterial (Variables|Default|GetBuilding_Floor28_StaticMeshComponent0) 0 "/Game/Y2/Models/Materials/PaintedNormals/BuildingFloor/Painted_BuildingFloor.Painted_BuildingFloor"))

(event Custom|BFBakedNormals
  ;[1 0.1543 0] Baked Normals
  (Rendering|Material|SetMaterial (Variables|Default|GetBuilding_Floor28_StaticMeshComponent0) 0 "/Game/Y2/Models/Materials/BakedNormals/Floor/N_Floor_BAKED.N_Floor_BAKED"))

(event Custom|BFImageNormals
  ;[0.3281 0.3281 0.3281] Image Normals
  (Rendering|Material|SetMaterial (Variables|Default|GetBuilding_Floor28_StaticMeshComponent0) 0 "/Game/Y2/Models/Materials/NBuilding_Floor.NBuilding_Floor"))

(event EventBeginPlay)

(event Collision|EventActorBeginOverlap
  (params (OtherActor :type Actor%20Object%20Reference)))

(event EventTick
  (params (DeltaSeconds :type Float%20%28single-precision%29)))

(fn ConstructionScript)