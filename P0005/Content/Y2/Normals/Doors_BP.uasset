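; Door Blueprint that swaps the materials on two door meshes to switch between normal map variants.
; Custom events set the handle metal, wood and glass slots on both meshes to either plain materials or image-normal versions.
; Baked and painted normal events exist but are empty, and BeginPlay, overlap and Tick are unused.
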(event Custom|DoorNonNormals
  (bind _door_v8_staticmeshcomponent0 (Variables|Default|GetDoor_V8_StaticMeshComponent0))
  ;[1 1 1] Non-Normals
  (Rendering|Material|SetMaterial _door_v8_staticmeshcomponent0 0 "/Game/3D-Models/Building/Door/Door_Handle_Metal.Door_Handle_Metal")
  (Rendering|Material|SetMaterial _door_v8_staticmeshcomponent0 1 "/Game/3D-Models/Building/Door/Door_Wood.Door_Wood")
  (Rendering|Material|SetMaterial (Variables|Default|GetDoor_V9_StaticMeshComponent0) 2 "/Game/3D-Models/Building/Door/Door_Glass.Door_Glass"))

(event Custom|DoorImageNormals
  (bind _door_v8_staticmeshcomponent0 (Variables|Default|GetDoor_V8_StaticMeshComponent0))
  ;[1 1 1] Image Normals
  (Rendering|Material|SetMaterial _door_v8_staticmeshcomponent0 0 "/Game/Y2/Models/Materials/NDoor_Handle_Metal.NDoor_Handle_Metal")
  (Rendering|Material|SetMaterial _door_v8_staticmeshcomponent0 1 "/Game/Y2/Models/Materials/NDoor_Wood.NDoor_Wood")
  (Rendering|Material|SetMaterial (Variables|Default|GetDoor_V9_StaticMeshComponent0) 2 "/Game/Y2/Models/Materials/NDoor_Glass.NDoor_Glass"))

(event Custom|DoorBakedNormals)

(event Custom|DoorPaintedNormals)

(event EventBeginPlay)

(event Collision|EventActorBeginOverlap
  (params (OtherActor :type Actor%20Object%20Reference)))

(event EventTick
  (params (DeltaSeconds :type Float%20%28single-precision%29)))

(fn ConstructionScript)