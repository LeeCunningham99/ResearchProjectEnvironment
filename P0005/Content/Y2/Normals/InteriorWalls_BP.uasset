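; Blueprint grouping interior building wall meshes that switches them between normal-map material variants.
; Four custom events (Painted, Non, Image and Baked Normals) each call SetMaterial on slots 0 and 1 of the same hard-wired wall components.
; Non and Image use a different material per slot, while Painted and Baked both apply N_WallInterior_BAKED to both slots, so their results are identical.
; Nothing in this Blueprint calls these events.
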(event Custom|IWBakedNormals
  (bind _building_wall104_staticmeshcomponent0 (Variables|Default|GetBuilding_Wall104_StaticMeshComponent0))
  ;[1 0.1543 0] Baked Normals
  (Rendering|Material|SetMaterial _building_wall104_staticmeshcomponent0 0 "/Game/Y2/Models/Materials/BakedNormals/WallInterior/N_WallInterior_BAKED.N_WallInterior_BAKED")
  (Rendering|Material|SetMaterial _building_wall104_staticmeshcomponent0 1 "/Game/Y2/Models/Materials/BakedNormals/Wall/N_WallInterior_BAKED.N_WallInterior_BAKED"))

(event Custom|IWNonNormals
  (bind _building_wall104_staticmeshcomponent0 (Variables|Default|GetBuilding_Wall104_StaticMeshComponent0))
  ;[1 1 1] Non-Normals
  (Rendering|Material|SetMaterial _building_wall104_staticmeshcomponent0 0 "/Game/3D-Models/Building/Wall_Interior_Mat.Wall_Interior_Mat")
  (Rendering|Material|SetMaterial _building_wall104_staticmeshcomponent0 1 "/Game/3D-Models/Building/Building_Wall_Interior.Building_Wall_Interior"))

(event Custom|IWImage%20Normals
  (bind _building_wall104_staticmeshcomponent0 (Variables|Default|GetBuilding_Wall104_StaticMeshComponent0))
  ;[0.3281 0.3281 0.3281] Image Normals
  (Rendering|Material|SetMaterial _building_wall104_staticmeshcomponent0 0 "/Game/Y2/Models/Materials/NWall_Interior_Mat.NWall_Interior_Mat")
  (Rendering|Material|SetMaterial _building_wall104_staticmeshcomponent0 1 "/Game/Y2/Models/Materials/NBuilding_Wall_Interior.NBuilding_Wall_Interior"))

(event Custom|IWPaintedNormals
  (bind _building_wall104_staticmeshcomponent0 (Variables|Default|GetBuilding_Wall104_StaticMeshComponent0))
  ;[0 1 0.001688] Painted Normals
  (Rendering|Material|SetMaterial _building_wall104_staticmeshcomponent0 0 "/Game/Y2/Models/Materials/BakedNormals/WallInterior/N_WallInterior_BAKED.N_WallInterior_BAKED")
  (Rendering|Material|SetMaterial _building_wall104_staticmeshcomponent0 1 "/Game/Y2/Models/Materials/BakedNormals/Wall/N_WallInterior_BAKED.N_WallInterior_BAKED"))

(event EventBeginPlay)

(event Collision|EventActorBeginOverlap
  (params (OtherActor :type Actor%20Object%20Reference)))

(event EventTick
  (params (DeltaSeconds :type Float%20%28single-precision%29)))

(fn ConstructionScript)