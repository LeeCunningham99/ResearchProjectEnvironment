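; Rocks_BP groups a set of rock static mesh components and switches their shared material, apparently to compare normal map variants.
; Custom events apply one material to slot 0 of every rock at once: RocksNonNormals sets Rock2 and RocksImageNormals sets NRockMaterial.
; RocksBakedNormals and RocksPaintedNormals are empty stubs, and nothing in this Blueprint calls the events.
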(event Custom|RocksNonNormals
  (Rendering|Material|SetMaterial (Variables|Default|GetRock24_StaticMeshComponent0) 0 "/Game/3D-Models/Rocks/Rock2.Rock2"))

(event Custom|RocksImageNormals
  (Rendering|Material|SetMaterial (Variables|Default|GetRock24_StaticMeshComponent0) 0 "/Game/Y2/Models/NRockMaterial.NRockMaterial"))

(event Custom|RocksBakedNormals)

(event Custom|RocksPaintedNormals)

(event EventBeginPlay)

(event Collision|EventActorBeginOverlap
  (params (OtherActor :type Actor%20Object%20Reference)))

(event EventTick
  (params (DeltaSeconds :type Float%20%28single-precision%29)))

(fn ConstructionScript)