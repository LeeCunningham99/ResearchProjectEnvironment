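; BuildingWindows_BP is an actor holding seven building window static meshes that switch between surface normal variants.
; Custom events set the material on slot 0 of every window mesh: one applies a plain non-normal material, another an image-based normal map version.
; Events for baked and painted normals exist but are empty, as are the default events and construction script.
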(event Custom|BWinNonNormals
  ;[1 1 1] Non-Normals
  (Rendering|Material|SetMaterial (Variables|Default|GetBuilding_Window2_StaticMeshComponent0) 0 "/Game/3D-Models/Building/Building_Window1.Building_Window1"))

(event Custom|BWinImageNormals
  ;[1 1 1] Image Normals
  (Rendering|Material|SetMaterial (Variables|Default|GetBuilding_Window2_StaticMeshComponent0) 0 "/Game/Y2/Models/Materials/NBuilding_Window.NBuilding_Window"))

(event Custom|BWinBakedNormals)

(event Custom|BWinPaintedNormals)

(event EventBeginPlay)

(event Collision|EventActorBeginOverlap
  (params (OtherActor :type Actor%20Object%20Reference)))

(event EventTick
  (params (DeltaSeconds :type Float%20%28single-precision%29)))

(fn ConstructionScript)