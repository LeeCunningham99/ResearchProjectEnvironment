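; CurbCurved_BP groups ten curved curb static mesh components and switches their concrete material between normal-map variants.
; Custom events apply one material to all ten pieces: CCNonNormals sets Curb_Concrete, and CCImageNormals sets NCurb_Concrete.
; The baked and painted normals events are empty stubs, and the construction script does nothing.
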(event Custom|CCNonNormals
  ;[1 1 1] Non-Normals
  (Rendering|Material|SetMaterial (Variables|Default|GetCurb_Curved10_StaticMeshComponent0) 0 "/Game/3D-Models/Curb/Curb_Concrete.Curb_Concrete"))

(event Custom|CCImageNormals
  (Rendering|Material|SetMaterial (Variables|Default|GetCurb_Curved10_StaticMeshComponent0) 0 "/Game/Y2/Models/Materials/NCurb_Concrete.NCurb_Concrete"))

(event Custom|CCBakedNormals)

(event Custom|CCPaintedNormals)

(event EventBeginPlay)

(event Collision|EventActorBeginOverlap
  (params (OtherActor :type Actor%20Object%20Reference)))

(event EventTick
  (params (DeltaSeconds :type Float%20%28single-precision%29)))

(fn ConstructionScript)