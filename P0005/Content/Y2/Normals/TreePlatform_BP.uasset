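; Tree platform Blueprint that switches the wood material on its many static mesh pieces between normal-map variants.
; Four custom events (painted, non-normal, image and baked normals) each set material slot 0 on the same hard-wired component list.
; Painted and baked events both apply N_TreePlatform_BAKED, so they give identical results.
; Nothing in this Blueprint calls these events; BeginPlay, Tick and the construction script are empty.
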(event Custom|TPNonNormals
  ;[1 1 1] Non-Normals
  (Rendering|Material|SetMaterial (Variables|Default|GetTree_Platform_V42_StaticMeshComponent0) 0 "/Game/3D-Models/Tree_Platform/Tree_Platform_Wood.Tree_Platform_Wood"))

(event Custom|TPBakedNormals
  ;[1 0.1543 0] Baked Normals
  (Rendering|Material|SetMaterial (Variables|Default|GetTree_Platform_V42_StaticMeshComponent0) 0 "/Game/Y2/Models/Materials/BakedNormals/TreePlatform/N_TreePlatform_BAKED.N_TreePlatform_BAKED"))

(event Custom|TPPaintedNormals
  ;[0 1 0.001688] Painted Normals
  (Rendering|Material|SetMaterial (Variables|Default|GetTree_Platform_V42_StaticMeshComponent0) 0 "/Game/Y2/Models/Materials/BakedNormals/TreePlatform/N_TreePlatform_BAKED.N_TreePlatform_BAKED"))

(event Custom|TPImageNormals
  ;[0.3281 0.3281 0.3281] Image Normals
  (Rendering|Material|SetMaterial (Variables|Default|GetTree_Platform_V42_StaticMeshComponent0) 0 "/Game/Y2/Models/Materials/NTree_Platform_Wood.NTree_Platform_Wood"))

(event EventBeginPlay)

(event Collision|EventActorBeginOverlap
  (params (OtherActor :type Actor%20Object%20Reference)))

(event EventTick
  (params (DeltaSeconds :type Float%20%28single-precision%29)))

(fn ConstructionScript)