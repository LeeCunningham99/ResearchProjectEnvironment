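; Actor grouping the building ceiling meshes, whose material can be switched between four normal-map variants: none, image, baked and painted.
; Each custom event sets material slot 0 on a hard-wired list of mesh components to its variant's material.
; The Baked and Painted events omit ceiling pieces 33 and 34, which the other two events include.
; Nothing in this Blueprint calls these events, and its construction script is empty.
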(event Custom|BCNonNormals
  ;[1 1 1] Non-Normals
  (Rendering|Material|SetMaterial (Variables|Default|GetBuilding_Ceiling45_StaticMeshComponent0) 0 "/Game/3D-Models/Building/Building_Ceiling1.Building_Ceiling1"))

(event Custom|BCBakedNormals
  ;[1 0.1543 0] Baked Normals
  (Rendering|Material|SetMaterial (Variables|Default|GetBuilding_Ceiling45_StaticMeshComponent0) 0 "/Game/Y2/Models/Materials/BakedNormals/Ceiling/N_Ceiling_BAKED.N_Ceiling_BAKED"))

(event Custom|BCPaintedNormals
  ;[0 1 0.001688] Painted Normals
  (Rendering|Material|SetMaterial (Variables|Default|GetBuilding_Ceiling45_StaticMeshComponent0) 0 "/Game/Y2/Models/Materials/PaintedNormals/BuildingCeiling/Painted_BuildingCeiling.Painted_BuildingCeiling"))

(event Custom|BCImageNormals
  ;[0.3281 0.3281 0.3281] Image Normals
  (Rendering|Material|SetMaterial (Variables|Default|GetBuilding_Ceiling45_StaticMeshComponent0) 0 "/Game/Y2/Models/Materials/NBuilding_Ceiling.NBuilding_Ceiling"))

(event EventBeginPlay)

(event Collision|EventActorBeginOverlap
  (params (OtherActor :type Actor%20Object%20Reference)))

(event EventTick
  (params (DeltaSeconds :type Float%20%28single-precision%29)))

(fn ConstructionScript)