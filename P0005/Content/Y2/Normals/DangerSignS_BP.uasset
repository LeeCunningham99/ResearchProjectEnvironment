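; Blueprint grouping six small danger sign static meshes whose materials switch between normal-map variants.
; Four custom events (non-normals, baked, image and painted normals) each set the metal and sign-face material slots on all six meshes.
; Image and painted events assign identical materials.
; Nothing in this graph calls the events; BeginPlay, Tick and the construction script are empty.
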(event Custom|DangerSSNonNormals
  ;[1 1 1] Non-Normals
  (Rendering|Material|SetMaterial (Variables|Default|GetDangerSignS_2_StaticMeshComponent0) 0 "/Game/3D-Models/Signs/SignMetal.SignMetal")
  (Rendering|Material|SetMaterial (Variables|Default|GetDangerSignS_2_StaticMeshComponent0) 1 "/Game/3D-Models/Signs/Danger1.Danger1"))

(event Custom|DangerSSBakedNormals
  ;[1 0.1543 0] Baked Normals
  (Rendering|Material|SetMaterial (Variables|Default|GetDangerSignS_2_StaticMeshComponent0) 0 "/Game/Y2/Models/Materials/BakedNormals/Lamp/N_Metal_BAKED.N_Metal_BAKED")
  (Rendering|Material|SetMaterial (Variables|Default|GetDangerSignS_2_StaticMeshComponent0) 1 "/Game/Y2/Models/Materials/BakedNormals/DangerSignS/N_DangerSignS_BAKED.N_DangerSignS_BAKED"))

(event Custom|DangerSSPaintedNormals
  ;[0 1 0.001688] Painted Normals
  (Rendering|Material|SetMaterial (Variables|Default|GetDangerSignS_2_StaticMeshComponent0) 0 "/Game/Y2/Models/Materials/NSignMetal.NSignMetal")
  (Rendering|Material|SetMaterial (Variables|Default|GetDangerSignS_2_StaticMeshComponent0) 1 "/Game/Y2/Models/Materials/NDanger.NDanger"))

(event Custom|DangerSSImageNormals
  ;[0.3281 0.3281 0.3281] Image Normals
  (Rendering|Material|SetMaterial (Variables|Default|GetDangerSignS_2_StaticMeshComponent0) 0 "/Game/Y2/Models/Materials/NSignMetal.NSignMetal")
  (Rendering|Material|SetMaterial (Variables|Default|GetDangerSignS_2_StaticMeshComponent0) 1 "/Game/Y2/Models/Materials/NDanger.NDanger"))

(event EventBeginPlay)

(event Collision|EventActorBeginOverlap
  (params (OtherActor :type Actor%20Object%20Reference)))

(event EventTick
  (params (DeltaSeconds :type Float%20%28single-precision%29)))

(fn ConstructionScript)