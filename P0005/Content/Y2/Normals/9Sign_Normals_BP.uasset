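; Blueprint actor for a group of five "9" sign meshes that switches between normal-map material variants, apparently for comparing normal techniques.
; Four custom events (non-normals, baked, image, painted) each set both material slots on every sign mesh, with no caller in this Blueprint.
; The painted event assigns the same baked materials as the baked event, so those two modes look identical.
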(event Custom|9SignNonNormals
  ;[1 1 1] Non-Normals
  (Rendering|Material|SetMaterial (Variables|Default|Get9Sign_StaticMeshComponent1) 0 "/Game/3D-Models/Signs/SignMetal.SignMetal")
  (Rendering|Material|SetMaterial (Variables|Default|Get9Sign_StaticMeshComponent1) 1 "/Game/3D-Models/Signs/Nine.Nine"))

(event Custom|9SignBakedNormals
  ;[1 0.1543 0] Baked Normals
  (Rendering|Material|SetMaterial (Variables|Default|Get9Sign_StaticMeshComponent1) 0 "/Game/Y2/Models/Materials/BakedNormals/DangerSignT/N_Metal_BAKED.N_Metal_BAKED")
  (Rendering|Material|SetMaterial (Variables|Default|Get9Sign_StaticMeshComponent1) 1 "/Game/Y2/Models/Materials/BakedNormals/NineSign/N_NineSign_BAKED.N_NineSign_BAKED"))

(event Custom|9SignPaintedNormals
  ;[0 1 0.001688] Painted Normals
  (Rendering|Material|SetMaterial (Variables|Default|Get9Sign_StaticMeshComponent1) 0 "/Game/Y2/Models/Materials/BakedNormals/DangerSignT/N_Metal_BAKED.N_Metal_BAKED")
  (Rendering|Material|SetMaterial (Variables|Default|Get9Sign_StaticMeshComponent1) 1 "/Game/Y2/Models/Materials/BakedNormals/NineSign/N_NineSign_BAKED.N_NineSign_BAKED"))

(event Custom|9SignImageNormals
  ;[0.3281 0.3281 0.3281] Image Normals
  (Rendering|Material|SetMaterial (Variables|Default|Get9Sign_StaticMeshComponent1) 0 "/Game/Y2/Models/Materials/NSignMetal.NSignMetal")
  (Rendering|Material|SetMaterial (Variables|Default|Get9Sign_StaticMeshComponent1) 1 "/Game/Y2/Models/Materials/N9plus.N9plus"))

(event EventBeginPlay)

(event Collision|EventActorBeginOverlap
  (params (OtherActor :type Actor%20Object%20Reference)))

(event EventTick
  (params (DeltaSeconds :type Float%20%28single-precision%29)))

(fn ConstructionScript)