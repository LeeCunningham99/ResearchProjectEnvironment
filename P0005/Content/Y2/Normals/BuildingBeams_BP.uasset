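; BuildingBeams_BP groups a building's wall beam meshes and switches their material, apparently to compare normal-map variants.
; BBNonNormals sets material slot 0 on the whole hardcoded set of beam components to Building_Wall_Beam1.
; BBImageNormals sets the same slot to NBuilding_Wall_Beam.
; BBBakedNormals and BBPaintedNormals are empty stubs, and nothing in this Blueprint calls these custom events.
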(event Custom|BBNonNormals
  ;[1 1 1] Non-Normals
  (Rendering|Material|SetMaterial (Variables|Default|GetBuilding_Wall_Beam187_StaticMeshComponent0) 0 "/Game/3D-Models/Building/Building_Wall_Beam1.Building_Wall_Beam1"))

(event Custom|BBImageNormals
  ;[1 1 1] Image Normals
  (Rendering|Material|SetMaterial (Variables|Default|GetBuilding_Wall_Beam187_StaticMeshComponent0) 0 "/Game/Y2/Models/Materials/NBuilding_Wall_Beam.NBuilding_Wall_Beam"))

(event Custom|BBBakedNormals)

(event Custom|BBPaintedNormals)

(event EventBeginPlay)

(event Collision|EventActorBeginOverlap
  (params (OtherActor :type Actor%20Object%20Reference)))

(event EventTick
  (params (DeltaSeconds :type Float%20%28single-precision%29)))

(fn ConstructionScript)