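; Tree Blueprint with three Gledista Triacanthos static mesh components that switches between material sets to show different normal map variants.
; Custom events set four material slots on all three meshes: Tree1NonNormals applies the base materials, Tree1ImageNormals the N-prefixed versions.
; Tree1BakedNormals and Tree1PaintedNormals are empty stubs, and nothing in this Blueprint calls the events.
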(event Custom|Tree1NonNormals
  (bind _1gledista_triacanthos2_staticmeshcomponent0 (Variables|Default|Get1Gledista_Triacanthos2_StaticMeshComponent0))
  ;[1 1 1] Non-Normals
  (Rendering|Material|SetMaterial _1gledista_triacanthos2_staticmeshcomponent0 0 "/Game/3D-Models/Tree/Material__6.Material__6")
  (Rendering|Material|SetMaterial _1gledista_triacanthos2_staticmeshcomponent0 1 "/Game/3D-Models/Tree/Material__8.Material__8")
  (Rendering|Material|SetMaterial _1gledista_triacanthos2_staticmeshcomponent0 2 "/Game/3D-Models/Tree/Material__14.Material__14")
  (Rendering|Material|SetMaterial _1gledista_triacanthos2_staticmeshcomponent0 3 "/Game/3D-Models/Tree/Material__5.Material__5"))

(event Custom|Tree1ImageNormals
  (bind _1gledista_triacanthos2_staticmeshcomponent0 (Variables|Default|Get1Gledista_Triacanthos2_StaticMeshComponent0))
  ;[1 1 1] Image Normals
  (Rendering|Material|SetMaterial _1gledista_triacanthos2_staticmeshcomponent0 0 "/Game/Y2/Models/Materials/NMaterial__6.NMaterial__6")
  (Rendering|Material|SetMaterial _1gledista_triacanthos2_staticmeshcomponent0 1 "/Game/Y2/Models/Materials/NMaterial__8.NMaterial__8")
  (Rendering|Material|SetMaterial _1gledista_triacanthos2_staticmeshcomponent0 2 "/Game/Y2/Models/Materials/NMaterial__14.NMaterial__14")
  (Rendering|Material|SetMaterial _1gledista_triacanthos2_staticmeshcomponent0 3 "/Game/Y2/Models/Materials/NMaterial__5.NMaterial__5"))

(event Custom|Tree1BakedNormals)

(event Custom|Tree1PaintedNormals)

(event EventBeginPlay)

(event Collision|EventActorBeginOverlap
  (params (OtherActor :type Actor%20Object%20Reference)))

(event EventTick
  (params (DeltaSeconds :type Float%20%28single-precision%29)))

(fn ConstructionScript)