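; Chain actor built from many static mesh link components, with events named for switching between normal-map variants of its material.
; ChainNonNormal and ChainImageNormal each set material slot 0 on the whole set of links in a single SetMaterial call.
; ChainBakedNormal and ChainPaintedNormal are empty stubs, and nothing in this Blueprint calls any of the events.
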(event Custom|ChainNonNormal
  ;[1 1 1] Non-Normal
  (Rendering|Material|SetMaterial (Variables|Default|GetChain_V16_StaticMeshComponent0) 0 "/Game/3D-Models/Chain/Material.Material"))

(event Custom|ChainImageNormal
  ;[1 1 1] Image Normals
  (Rendering|Material|SetMaterial (Variables|Default|GetChain_V16_StaticMeshComponent0) 0 "/Game/3D-Models/Chain/Material.Material"))

(event Custom|ChainBakedNormal)

(event Custom|ChainPaintedNormal)

(event EventBeginPlay)

(event Collision|EventActorBeginOverlap
  (params (OtherActor :type Actor%20Object%20Reference)))

(event EventTick
  (params (DeltaSeconds :type Float%20%28single-precision%29)))

(fn ConstructionScript)