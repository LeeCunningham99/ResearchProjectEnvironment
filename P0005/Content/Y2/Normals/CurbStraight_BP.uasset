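; Blueprint grouping straight curb mesh components, with custom events that switch their material between normal-map variants.
; CSNonNormals, CSImageNormals, CSBakedNormals and CSPaintedNormals each set material slot 0 on every curb piece.
; CSPaintedNormals applies the same baked material as CSBakedNormals, so those two variants are identical.
; Nothing in this Blueprint calls the events, and its construction script is empty.
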(event Custom|CSNonNormals
  ;[1 1 1] Non-Normals
  (Rendering|Material|SetMaterial (Variables|Default|GetCurb_Straight63_StaticMeshComponent0) 0 "/Game/3D-Models/Curb/Curb_Concrete.Curb_Concrete"))

(event Custom|CSBakedNormals
  ;[1 0.1543 0] Baked Normals
  (Rendering|Material|SetMaterial (Variables|Default|GetCurb_Straight63_StaticMeshComponent0) 0 "/Game/Y2/Models/Materials/BakedNormals/CurbStraight/N_CurbStraight_BAKED.N_CurbStraight_BAKED"))

(event Custom|CSPaintedNormals
  ;[0 1 0.001688] Painted Normals
  (Rendering|Material|SetMaterial (Variables|Default|GetCurb_Straight63_StaticMeshComponent0) 0 "/Game/Y2/Models/Materials/BakedNormals/CurbStraight/N_CurbStraight_BAKED.N_CurbStraight_BAKED"))

(event Custom|CSImageNormals
  ;[0.3281 0.3281 0.3281] Image Normals
  (Rendering|Material|SetMaterial (Variables|Default|GetCurb_Straight63_StaticMeshComponent0) 0 "/Game/Y2/Models/Materials/NCurb_Concrete.NCurb_Concrete"))

(event EventBeginPlay)

(event Collision|EventActorBeginOverlap
  (params (OtherActor :type Actor%20Object%20Reference)))

(event EventTick
  (params (DeltaSeconds :type Float%20%28single-precision%29)))

(fn ConstructionScript)