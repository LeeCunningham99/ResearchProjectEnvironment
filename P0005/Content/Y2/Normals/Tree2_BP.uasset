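; Tree2_BP is a Blueprint grouping Gleditsia triacanthos tree meshes whose materials switch between normal-map variants, apparently for comparing them.
; Tree2NonNormals and Tree2ImageNormals each set three material slots on every listed mesh component, using the plain or N-prefixed material set respectively.
; Tree2BakedNormals and Tree2PaintedNormals are empty stubs.
; Nothing here calls these events, so switching relies on an external trigger.
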(event Custom|Tree2NonNormals
  ;[1 1 1] Non-Normals
  (Rendering|Material|SetMaterial (Variables|Default|Get2Gledista_Triacanthos_74_StaticMeshComponent0) 0 "/Game/3D-Models/Tree/Material__6.Material__6")
  (Rendering|Material|SetMaterial (Variables|Default|Get2Gledista_Triacanthos_74_StaticMeshComponent0) 1 "/Game/3D-Models/Tree/Material__8.Material__8")
  (Rendering|Material|SetMaterial (Variables|Default|Get2Gledista_Triacanthos_74_StaticMeshComponent0) 2 "/Game/3D-Models/Tree/Material__5.Material__5"))

(event Custom|Tree2ImageNormals
  ;[1 1 1] Image Normals
  (Rendering|Material|SetMaterial (Variables|Default|Get2Gledista_Triacanthos_74_StaticMeshComponent0) 0 "/Game/Y2/Models/Materials/NMaterial__6.NMaterial__6")
  (Rendering|Material|SetMaterial (Variables|Default|Get2Gledista_Triacanthos_74_StaticMeshComponent0) 1 "/Game/Y2/Models/Materials/NMaterial__8.NMaterial__8")
  (Rendering|Material|SetMaterial (Variables|Default|Get2Gledista_Triacanthos_74_StaticMeshComponent0) 2 "/Game/Y2/Models/Materials/NMaterial__5.NMaterial__5"))

(event Custom|Tree2BakedNormals)

(event Custom|Tree2PaintedNormals)

(event EventBeginPlay)

(event Collision|EventActorBeginOverlap
  (params (OtherActor :type Actor%20Object%20Reference)))

(event EventTick
  (params (DeltaSeconds :type Float%20%28single-precision%29)))

(fn ConstructionScript)