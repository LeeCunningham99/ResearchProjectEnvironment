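; Blueprint grouping 24 building light meshes, with custom events that switch their materials between normal-map variants.
; BLNonNormals applies the plain glass, bulb and metal materials across every mesh's three slots.
; BLImageNormals applies N-prefixed glass and metal materials but keeps the same bulb material.
; BLBakedNormals and BLPaintedNormals are empty, and nothing in this Blueprint calls the switch events.
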(event Custom|BLImageNormals
  ;[1 1 1] Non-Normals
  (Rendering|Material|SetMaterial (Variables|Default|GetBuilding_Light21_StaticMeshComponent0) 0 "/Game/Y2/Models/Materials/NBuilding_Light_Glass.NBuilding_Light_Glass")
  (Rendering|Material|SetMaterial (Variables|Default|GetBuilding_Light21_StaticMeshComponent0) 1 "/Game/3D-Models/Building/Light/Building_Light_Bulbs.Building_Light_Bulbs")
  (Rendering|Material|SetMaterial (Variables|Default|GetBuilding_Light21_StaticMeshComponent0) 2 "/Game/Y2/Models/Materials/NBuilding_Light_Metal.NBuilding_Light_Metal"))

(event Custom|BLNonNormals
  ;[1 1 1] Non-Normals
  (Rendering|Material|SetMaterial (Variables|Default|GetBuilding_Light21_StaticMeshComponent0) 0 "/Game/3D-Models/Building/Light/Building_Light_Glass.Building_Light_Glass")
  (Rendering|Material|SetMaterial (Variables|Default|GetBuilding_Light21_StaticMeshComponent0) 1 "/Game/3D-Models/Building/Light/Building_Light_Bulbs.Building_Light_Bulbs")
  (Rendering|Material|SetMaterial (Variables|Default|GetBuilding_Light21_StaticMeshComponent0) 2 "/Game/3D-Models/Building/Light/Building_Light_Metal.Building_Light_Metal"))

(event Custom|BLBakedNormals)

(event Custom|BLPaintedNormals)

(event EventBeginPlay)

(event Collision|EventActorBeginOverlap
  (params (OtherActor :type Actor%20Object%20Reference)))

(event EventTick
  (params (DeltaSeconds :type Float%20%28single-precision%29)))

(fn ConstructionScript)