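; Sign actor for a "16" sign that swaps its materials between normal-map variants, apparently for comparing normal techniques.
; Four custom events (non-normals, baked, image and painted) each set the metal and sixteen-face material slots on four static mesh components.
; The painted event assigns the same baked materials as the baked event.
; Nothing in the Blueprint calls these events, and its construction script is empty.
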(event Custom|16SignNonNormals
  ;[1 1 1] Non-Normals
  (Rendering|Material|SetMaterial (Variables|Default|Get16Sign_StaticMeshComponent1) 0 "/Game/3D-Models/Signs/SignMetal.SignMetal")
  (Rendering|Material|SetMaterial (Variables|Default|Get16Sign_StaticMeshComponent1) 1 "/Game/3D-Models/Signs/Sixteen.Sixteen"))

(event Custom|16SignBakedNormals
  ;[1 0.1543 0] Baked Normals
  (Rendering|Material|SetMaterial (Variables|Default|Get16Sign_StaticMeshComponent1) 0 "/Game/Y2/Models/Materials/BakedNormals/DangerSignT/N_Metal_BAKED.N_Metal_BAKED")
  (Rendering|Material|SetMaterial (Variables|Default|Get16Sign_StaticMeshComponent1) 1 "/Game/Y2/Models/Materials/BakedNormals/SixteenSign/N_SixteenSign_BAKED.N_SixteenSign_BAKED"))

(event Custom|16SignPaintedNormals
  ;[0 1 0.001688] Painted Normals
  (Rendering|Material|SetMaterial (Variables|Default|Get16Sign_StaticMeshComponent1) 0 "/Game/Y2/Models/Materials/BakedNormals/DangerSignT/N_Metal_BAKED.N_Metal_BAKED")
  (Rendering|Material|SetMaterial (Variables|Default|Get16Sign_StaticMeshComponent1) 1 "/Game/Y2/Models/Materials/BakedNormals/SixteenSign/N_SixteenSign_BAKED.N_SixteenSign_BAKED"))

(event Custom|16SignImageNormals
  ;[0.3281 0.3281 0.3281] Image Normals
  (Rendering|Material|SetMaterial (Variables|Default|Get16Sign_StaticMeshComponent1) 0 "/Game/Y2/Models/Materials/NSignMetal.NSignMetal")
  (Rendering|Material|SetMaterial (Variables|Default|Get16Sign_StaticMeshComponent1) 1 "/Game/Y2/Models/Materials/NSixteen.NSixteen"))

(event EventBeginPlay)

(event Collision|EventActorBeginOverlap
  (params (OtherActor :type Actor%20Object%20Reference)))

(event EventTick
  (params (DeltaSeconds :type Float%20%28single-precision%29)))

(fn ConstructionScript)