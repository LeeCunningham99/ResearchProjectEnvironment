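; Elevator actor that runs a timed ride sequence when something overlaps its box or ElevatorFunctionality is called.
; IsMovingUp alternates each trigger between running the sequence and only clearing the flag.
; Three timelines, chained from Update pins through fixed delays with sounds, move the door, shift the elevator vertically, reopen the door, then set EComplete.
; A disconnected copy of the sequence with extra state flags never runs.
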(event OnComponentBeginOverlap(Box)
  (params (OverlappedComponent :type Primitive%20Component%20Object%20Reference) (OtherActor :type Actor%20Object%20Reference) (OtherComp :type Primitive%20Component%20Object%20Reference) (OtherBodyIndex :type Integer) (bFromSweep :type Boolean) (SweepResult :type Hit%20Result%20Structure%20%28by%20ref%29))
  (if (Variables|Default|GetIsMovingUp?)
    (Variables|Default|SetIsMovingUp? false)
    (else
      (Variables|Default|SetIsMovingUp? true)
      (Utilities|FlowControl|Delay 2.0)
      (Audio|PlaySound2D 0 1.0 1.0 0.0 0 0)
      (bind _dooropenclose (Timeline|ElevatorDoor Play)
        (:Update
          (Transformation|SetRelativeLocation (Variables|Default|GetDoor) (Math|Vector|MakeVector 88.0 140.9 _dooropenclose) false false)
          (Utilities|FlowControl|Delay 4.0)
          (Audio|PlaySound2D 0 1.0 1.0 0.0 0 0)
          (bind _updown (Timeline|ElevatorUpDown Play)
            (:Update
              (Transformation|SetRelativeLocation (Variables|Default|GetElevator) (Math|Vector|MakeVector 0.0 0.0 _updown) false false)
              (Utilities|FlowControl|Delay 1e+01)
              (Audio|PlaySound2D 0 1.0 1.0 0.0 0 0)
              (bind _open (Timeline|DoorOpen Play)
                (:Update
                  (Transformation|SetRelativeLocation (Variables|Default|GetDoor) (Math|Vector|MakeVector 88.0 140.9 _open) false false)
                  (Variables|Default|SetEComplete true))))))))))

(event Custom|Elevator%20Functionality
  (if (Variables|Default|GetIsMovingUp?)
    (Variables|Default|SetIsMovingUp? false)
    (else
      (Variables|Default|SetIsMovingUp? true)
      (Utilities|FlowControl|Delay 2.0)
      (Audio|PlaySound2D 0 1.0 1.0 0.0 0 0)
      (bind _dooropenclose (Timeline|ElevatorDoor Play)
        (:Update
          (Transformation|SetRelativeLocation (Variables|Default|GetDoor) (Math|Vector|MakeVector 88.0 140.9 _dooropenclose) false false)
          (Utilities|FlowControl|Delay 4.0)
          (Audio|PlaySound2D 0 1.0 1.0 0.0 0 0)
          (bind _updown (Timeline|ElevatorUpDown Play)
            (:Update
              (Transformation|SetRelativeLocation (Variables|Default|GetElevator) (Math|Vector|MakeVector 0.0 0.0 _updown) false false)
              (Utilities|FlowControl|Delay 1e+01)
              (Audio|PlaySound2D 0 1.0 1.0 0.0 0 0)
              (bind _open (Timeline|DoorOpen Play)
                (:Update
                  (Transformation|SetRelativeLocation (Variables|Default|GetDoor) (Math|Vector|MakeVector 88.0 140.9 _open) false false)
                  (Variables|Default|SetEComplete true))))))))))

(event EventBeginPlay)

(event Collision|EventActorBeginOverlap
  (params (OtherActor :type Actor%20Object%20Reference)))

(event EventTick
  (params (DeltaSeconds :type Float%20%28single-precision%29)))

(fn ConstructionScript)