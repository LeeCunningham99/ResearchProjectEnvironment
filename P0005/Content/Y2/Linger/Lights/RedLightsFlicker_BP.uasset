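; Red lights Blueprint meant to flicker a set of lights, left and right by their names, though none of its logic is connected.
; Disconnected nodes play slow, medium and fast timelines on separate light groups; slow and medium feed track values into intensity, while fast sets intensity to zero.
; BeginPlay, the RedLightsFlicker event and the construction script are empty, so the graph changes no lights as it stands.
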(event Custom|RedLightsFlicker)

(event EventBeginPlay)

(fn ConstructionScript)