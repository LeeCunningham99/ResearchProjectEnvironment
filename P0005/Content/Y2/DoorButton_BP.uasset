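; Door button actor that opens every SlidingDoor_BP in the level, triggered by the F interact input or any overlap with its Box.
; It plays a sound, waits briefly, then DoorScanner swaps the red light for the green before all doors are opened.
; A delayed GreenLightFlicker event drives the green light's intensity through a timeline.
; The Interact event is empty and the button-movement animation is unconnected.
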(event OnComponentBeginOverlap(Box)
  (params (OverlappedComponent :type Primitive%20Component%20Object%20Reference) (OtherActor :type Actor%20Object%20Reference) (OtherComp :type Primitive%20Component%20Object%20Reference) (OtherBodyIndex :type Integer) (bFromSweep :type Boolean) (SweepResult :type Hit%20Result%20Structure%20%28by%20ref%29))
  (Audio|PlaySound2D 0 1.0 1.0 0.0 0 0)
  (Utilities|FlowControl|Delay 3.0)
  (CallFunction|DoorScanner)
  (bind _outactors (Actor|GetAllActorsOfClass "/Game/Y2/SlidingDoor_BP.SlidingDoor_BP_C"))
  (bind _array_element (Utilities|Array|ForEachLoopwithBreak _outactors)
    (:LoopBody
      (Default|OpenSlidingDoor _array_element)
      (Utilities|FlowControl|Delay 2.0)
      (CallFunction|GreenLightFlicker))))

(event Custom|GreenLightFlicker
  (bind _green (Timeline|GreenLightFlickering Play)
    (:Update
      (Rendering|Components|Light|SetIntensity (Variables|Default|GetGreenLight) _green))))

(event Input|EnhancedActionEvents|EnhancedInputActionIA_Interact_F
  (params (ActionValue :type Boolean) (ElapsedSeconds :type Float%20%28double-precision%29) (TriggeredSeconds :type Float%20%28double-precision%29) (InputAction :type Input%20Action%20Object%20Reference :default "/Game/FirstPerson/Input/Actions/IA_Interact_F.IA_Interact_F"))
  (:Started
    (Audio|PlaySound2D 0 1.0 1.0 0.0 0 0)
    (Utilities|FlowControl|Delay 3.0)
    (CallFunction|DoorScanner)
    (bind _outactors (Actor|GetAllActorsOfClass "/Game/Y2/SlidingDoor_BP.SlidingDoor_BP_C"))
    (bind _array_element (Utilities|Array|ForEachLoopwithBreak _outactors)
      (:LoopBody
        (Default|OpenSlidingDoor _array_element)
        (Utilities|FlowControl|Delay 2.0)
        (CallFunction|GreenLightFlicker)))))

(event EventBeginPlay)

(event Collision|EventActorBeginOverlap
  (params (OtherActor :type Actor%20Object%20Reference)))

(event EventTick
  (params (DeltaSeconds :type Float%20%28single-precision%29)))

(event EventInteract)

(fn ConstructionScript)

(fn DoorScanner
  (Rendering|SetVisibility (Variables|Default|GetRedLight) false false)
  (Rendering|SetVisibility (Variables|Default|GetGreenLight) true false))